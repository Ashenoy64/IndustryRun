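; Player controller that owns the in-game HUD and pause menu widgets and switches between them.
; BeginPlay creates both widgets, shows the HUD and sets game-only input.
; Pressing P pauses the game and swaps to the pause widget with UI input and cursor; UnPause swaps back and hides the cursor, without itself unpausing the game.
; A Score event writes the current and high score into HUD text.
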(event Custom|Score
  (params (Score :type Integer64) (HighScore :type Integer64))
  (bind _hud (Variables|Default|GetHUD))
  (Variables|/Script/UMG.TextBlock|SetText (Variables|/Game/Content/UI/HUD.HUD_C|GetScore _hud) (Utilities|Text|FormatText "{score}" Score))
  (Variables|/Script/UMG.TextBlock|SetText (Variables|/Game/Content/UI/HUD.HUD_C|GetHighScore _hud) (Utilities|Text|FormatText "HighScore:{score}" HighScore)))

(event Custom|UnPause
  (Widget|RemovefromParent (Variables|Default|GetPauseWidget))
  (UserInterface|Viewport|AddtoViewport (Variables|Default|GetHUD) 0)
  (Input|SetInputModeGameOnly self false)
  (Variables|Default|SetbShowMouseCursor false))

(event EventBeginPlay
  (bind _returnvalue (UserInterface|CreateWidget "/Game/Content/UI/HUD.HUD_C"))
  (bind _output_get (Variables|Default|SetHUD _returnvalue))
  (bind _returnvalue_2 (UserInterface|CreateWidget "/Game/Content/UI/BP_Pause.BP_Pause_C"))
  (Variables|Default|SetPauseWidget _returnvalue_2)
  (UserInterface|Viewport|AddtoViewport _output_get 0)
  (Input|SetInputModeGameOnly self false))

(event Input|KeyboardEvents|P
  (params (Key :type Key%20Structure :default "None"))
  (:Pressed
    (Game|SetGamePaused true)
    (Widget|RemovefromParent (Variables|Default|GetHUD))
    (UserInterface|Viewport|AddtoViewport (Variables|Default|GetPauseWidget) 0)
    (Input|SetInputModeUIOnly self 0 "LockInFullscreen" false)
    (Variables|Default|SetbShowMouseCursor true)))

(fn ConstructionScript)