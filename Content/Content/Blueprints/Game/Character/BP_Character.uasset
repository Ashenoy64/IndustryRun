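; Player character for a three-lane dodging game that jumps and switches lanes to avoid obstacles.
; Left and Right keys update the lane stored in the GameState, and Tick slides the character's Y toward it at constant speed with a swept move and fixed X.
; The first obstacle hit sends the score to the GameInstance, stops the score timer, ragdolls the character and opens the end-game level after a delay.
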(event Custom|RagDoll
  (Physics|SetSimulatePhysics (Variables|Character|GetMesh) true)
  (Pawn|Components|CharacterMovement|DisableMovement (Variables|Character|GetCharacterMovement)))

(event EventBeginPlay
  (bind _asbp_game_state (Utilities|Casting|CastToBP_GameState (Game|GetGameState)))
  (Variables|Default|SetGameState _asbp_game_state))

(event Collision|EventActorBeginOverlap
  (params (OtherActor :type Actor%20Object%20Reference)))

(event Collision|EventHit
  (params (MyComp :type Primitive%20Component%20Object%20Reference) (Other :type Actor%20Object%20Reference) (OtherComp :type Primitive%20Component%20Object%20Reference) (bSelfMoved :type Boolean) (HitLocation :type Vector :default "0, 0, 0") (HitNormal :type Vector :default "0, 0, 0") (NormalImpulse :type Vector :default "0, 0, 0") (Hit :type Hit%20Result%20Structure%20%28by%20ref%29))
  (bind _gamestate (Variables|Default|GetGameState))
  (Utilities|Casting|CastToObstacleBase Other)
  (Utilities|FlowControl|DoOnce false
    (:Completed
      (bind _asbp_game_instance (Utilities|Casting|CastToBP_GameInstance (Game|GetGameInstance)))
      (Default|CharacterEnd _asbp_game_instance (Variables|/Game/Content/Blueprints/Game/BP_GameState.BP_GameState_C|GetScore _gamestate))
      (Utilities|Time|ClearandInvalidateTimerbyHandle (Variables|/Game/Content/Blueprints/Game/BP_GameState.BP_GameState_C|GetScoreTimer _gamestate))
      (CallFunction|RagDoll)
      (Utilities|FlowControl|Delay 2.0)
      (Game|OpenLevel(byObjectReference) "/Game/Maps/EndGame.EndGame"))))

(event EventTick
  (params (DeltaSeconds :type Float%20%28single-precision%29))
  (bind _returnvalue (Transformation|GetActorLocation))
  (Transformation|SetActorLocation (Math|Vector|MakeVector 2.2e+02 (Math|Interpolation|FInterptoConstant (.y _returnvalue) (Variables|Default|GetTargetLocation) DeltaSeconds (Variables|Default|GetSideWaysSpeed)) (.z _returnvalue)) true false))

(event Input|KeyboardEvents|Right
  (params (Key :type Key%20Structure :default "None"))
  (bind _gamestate (Variables|Default|GetGameState))
  (bind _right (Variables|/Game/Content/Blueprints/Game/BP_GameState.BP_GameState_C|GetRight _gamestate))
  (:Pressed
    (Variables|Default|SetTargetLocation (Utilities|Select :Index (Variables|/Game/Content/Blueprints/Game/BP_GameState.BP_GameState_C|GetSide _gamestate) :NewEnumerator0 _right :NewEnumerator1 (Variables|/Game/Content/Blueprints/Game/BP_GameState.BP_GameState_C|GetMiddle _gamestate) :NewEnumerator2 _right))
    (Variables|/Game/Content/Blueprints/Game/BP_GameState.BP_GameState_C|SetSide (Variables|Default|GetGameState) (Utilities|Select :Index (Variables|/Game/Content/Blueprints/Game/BP_GameState.BP_GameState_C|GetSide _gamestate) :NewEnumerator0 "NewEnumerator2" :NewEnumerator1 "NewEnumerator0" :NewEnumerator2 "NewEnumerator2"))))

(event Input|KeyboardEvents|Left
  (params (Key :type Key%20Structure :default "None"))
  (bind _gamestate (Variables|Default|GetGameState))
  (bind _left (Variables|/Game/Content/Blueprints/Game/BP_GameState.BP_GameState_C|GetLeft _gamestate))
  (:Pressed
    (Variables|Default|SetTargetLocation (Utilities|Select :Index (Variables|/Game/Content/Blueprints/Game/BP_GameState.BP_GameState_C|GetSide _gamestate) :NewEnumerator0 _left :NewEnumerator1 _left :NewEnumerator2 (Variables|/Game/Content/Blueprints/Game/BP_GameState.BP_GameState_C|GetMiddle _gamestate)))
    (Variables|/Game/Content/Blueprints/Game/BP_GameState.BP_GameState_C|SetSide (Variables|Default|GetGameState) (Utilities|Select :Index (Variables|/Game/Content/Blueprints/Game/BP_GameState.BP_GameState_C|GetSide _gamestate) :NewEnumerator0 "NewEnumerator1" :NewEnumerator1 "NewEnumerator1" :NewEnumerator2 "NewEnumerator0"))))

(event Input|KeyboardEvents|SpaceBar
  (params (Key :type Key%20Structure :default "None"))
  (:Pressed
    (Character|Jump)
    (Variables|Default|SetJumping true)
    (Utilities|FlowControl|Delay 0.2)
    (Character|StopJumping)
    (Variables|Default|SetJumping false)))

(fn ConstructionScript)