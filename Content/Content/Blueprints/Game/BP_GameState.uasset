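; BP_GameState tracks the running score and high score and drives the game's speed ramp.
; On BeginPlay it resets the start speed and loads the high score from BP_GameInstance, then starts a looping timer that raises the score.
; Each tick of that timer updates the local high score, passes both values to BP_PlayerController, and asks the game instance to increase speed at regular score milestones.
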(event Custom|IncreseScore
  (bind _output_get (Variables|Default|SetScore (+ (Variables|Default|GetScore) 2)))
  (if (> _output_get (Variables|Default|GetHighScore))
    (Variables|Default|SetHighScore _output_get))
  (bind _asbp_player_controller (Utilities|Casting|CastToBP_PlayerController (Game|GetPlayerController 0)))
  (Default|Score _asbp_player_controller (Variables|Default|GetScore) (Variables|Default|GetHighScore))
  (if (== (Math|Integer|%(Integer) (Math|Conversions|ToInteger(Byte) _output_get) 50) 0)
    (Default|IncreaseGameSpeed (Variables|Default|GetAs%20BP%20Game%20Instance))))

(event EventBeginPlay
  (bind _output_get (Variables|Default|SetAs%20BP%20Game%20Instance (.AsBP%20Game%20Instance (Utilities|Casting|CastToBP_GameInstance (Game|GetGameInstance)))))
  (Default|SetStartSpeed _output_get)
  (bind _returnvalue (Utilities|Time|SetTimerbyFunctionName 0 "IncreseScore" 0.5 true))
  (Variables|Default|SetScoreTimer _returnvalue)
  (Variables|Default|SetHighScore (Variables|/Game/Content/Blueprints/BP_GameInstance.BP_GameInstance_C|GetHighScore _output_get)))

(fn ConstructionScript)